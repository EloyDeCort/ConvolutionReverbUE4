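; Player character with axis-driven movement and look (optional inverted Y) that carries and controls a dynamic audio source ball.
; Holding Carry traces from the camera and grabs the ball with a physics handle that follows a grab point each tick; physics simulates only while held.
; Other inputs switch or pause samples on the tagged source cached at BeginPlay, or quit.
; WAV recording nodes remain but are disconnected.
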(event `self.ReceiveBeginPlay`
  ;[0.5906 1 0.2582] Set Source Ball Etc
  (bind _outactors (`GameplayStatics.GetAllActorsWithTag` "AudioSource"))
  (bind _asbp_dynamic_audio_source (cast `/Game/Blueprints/BP_DynamicAudioSource` (`|GetArrayItem` _outactors)))
  (set `self.AudioSource` _asbp_dynamic_audio_source))

(event `InputAxis|MoveForward`
  (params (AxisValue :type "Float (single-precision)"))
  ;[0.5906 1 0.2582] Basic Movement
  (`self.AddMovementInput` (`self.GetActorForwardVector`) AxisValue))

(event `InputAxis|MoveRight`
  (params (AxisValue :type "Float (single-precision)"))
  ;[0.5906 1 0.2582] Basic Movement
  (`self.AddMovementInput` (`self.GetActorRightVector`) AxisValue))

(event `InputAxis|LookHorizontal`
  (params (AxisValue :type "Float (single-precision)"))
  ;[0.5906 1 0.2582] LookAt
  (`self.AddControllerYawInput` AxisValue))

(event `InputAxis|LookVertical`
  (params (AxisValue :type "Float (single-precision)"))
  ;[0.5906 1 0.2582] LookAt
  (if (`self.InvertedY`)
    (`self.AddControllerPitchInput` AxisValue)
    (else
      (`self.AddControllerPitchInput` (* AxisValue -1.0)))))

(event `InputAction|Exit`
  (params (Key :type "Key Structure"))
  ;[0.5906 1 0.2582] Quit Game
  (:`Pressed`
    (`KismetSystemLibrary.QuitGame` null "Quit")))

(event `Pick Up`
  (bind _camera (`self.Camera`))
  (bind _returnvalue (`SceneComponent.K2_GetComponentLocation` _camera))
  ;[1 0.5395 0.3864] Pick Up / Hold Source Ball
  (bind (_outhit _returnvalue_2) (`KismetSystemLibrary.LineTraceSingleForObjects` _returnvalue (+ _returnvalue (* (`SceneComponent.GetForwardVector` _camera) (`self.LookRange`))) (`|MakeArray` "ObjectTypeQuery7" :!type "EObjectTypeQuery Enum")))
  (if _returnvalue_2
    (bind (_bblockinghit _binitialoverlap _time _distance _location _impactpoint _normal _impactnormal _physmat _hitactor _hitcomponent) (`GameplayStatics.BreakHitResult` _outhit))
    (`PhysicsHandleComponent.GrabComponentAtLocation` (`self.PhysicsHandle`) _hitcomponent "None" (`self.K2_GetActorLocation` _hitactor))
    (bind _asbp_dynamic_audio_source (cast `/Game/Blueprints/BP_DynamicAudioSource` _hitactor))
    (set `self.Actor` _asbp_dynamic_audio_source)
    (`PrimitiveComponent.SetSimulatePhysics` (`/Game/Blueprints/BP_DynamicAudioSource.Sphere` _asbp_dynamic_audio_source) true)))

(event `InputAction|NextSample`
  (params (Key :type "Key Structure"))
  (bind _audiosource (`self.AudioSource`))
  ;[0.624 0.8714 1] Next / Previous Sample
  (:`Pressed`
    (`/Engine/EditorBlueprintResources/StandardMacros.IsValid` _audiosource
      (:`Is Valid`
        (`/Game/Blueprints/BP_DynamicAudioSource.NextSample` _audiosource)))))

(event `InputAction|Pause`
  (params (Key :type "Key Structure"))
  ;[0.624 0.8714 1] Pause Sample
  (:`Pressed`
    (bind _output_get (set `self.Paused` (not (`self.Paused`))))
    (`/Game/Blueprints/BP_DynamicAudioSource.Pause` (`self.AudioSource`) _output_get)))

(event `InputAction|PreviousSample`
  (params (Key :type "Key Structure"))
  (bind _audiosource (`self.AudioSource`))
  ;[0.624 0.8714 1] Next / Previous Sample
  (:`Pressed`
    (`/Engine/EditorBlueprintResources/StandardMacros.IsValid` _audiosource
      (:`Is Valid`
        (`/Game/Blueprints/BP_DynamicAudioSource.PreviousSample` _audiosource)))))

(event `Drop`
  (bind _actor (`self.Actor`))
  ;[1 0.5395 0.3864] Drop Source Ball
  (`PhysicsHandleComponent.ReleaseComponent` (`self.PhysicsHandle`))
  (`/Engine/EditorBlueprintResources/StandardMacros.IsValid` _actor
    (:`Is Valid`
      (`PrimitiveComponent.SetSimulatePhysics` (`/Game/Blueprints/BP_DynamicAudioSource.Sphere` _actor) false))))

(event `InputAction|Carry`
  (params (Key :type "Key Structure"))
  ;[1 0.5395 0.3864] Input for carrying
  (:`Pressed`
    (`self.Pick Up`))
  (:`Released`
    (`self.Drop`)))

(event `self.ReceiveTick`
  (params (DeltaSeconds :type "Float (single-precision)"))
  ;[1 0.5395 0.3864] Set Location of Ball when holding
  (`PhysicsHandleComponent.SetTargetLocation` (`self.PhysicsHandle`) (`SceneComponent.K2_GetComponentLocation` (`self.GrabLocation`))))

(event `Key|O`
  (params (Key :type "Key Structure"))
  ;[1 1 1] Recording to files (not used in ship build)
)

(event `Key|P`
  (params (Key :type "Key Structure"))
  ;[1 1 1] Recording to files (not used in ship build)
)

(fn `UserConstructionScript`)