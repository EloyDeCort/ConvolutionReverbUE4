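; BP_DynamicAudioSource is an audio source actor that plays one sound from a Samples list and displays its name on a text element.
; BeginPlay sets the first sample and creates a dynamic material from MI_AudioSource for the sphere.
; NextSample and PreviousSample step through the list with wraparound, updating sound and label and giving the sphere a random-hue emissive glow.
; Pause toggles the audio's paused state from its input.
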(event `self.ReceiveBeginPlay`
  ;[1 1 1] Creating Dynamic Material & Setting the sample to play
  (`AudioComponent.SetSound` (`self.Audio`) (`|GetArrayItem` (`self.Samples`)))
  (bind _returnvalue (`KismetMaterialLibrary.CreateDynamicMaterialInstance` "/Game/Materials/MI_AudioSource.MI_AudioSource"))
  (bind _output_get (set `self.DynMaterial` _returnvalue))
  (`PrimitiveComponent.SetMaterial` (`self.Sphere`) 0 _output_get)
  (bind _name (`self.GetSampleName`))
  (`/Game/Blueprints/BP_SampleTextActor.SetText` (`self.TextActor`) _name))

(fn `GetSampleName`
  (returns (Name :type String))
  (return (`KismetSystemLibrary.GetDisplayName` (`|GetArrayItem` (`self.Samples`) (`self.CurrentSampleIDX`)))))

(fn `NextSample`
  (bind _color (`self.Color`))
  (bind _result (`/Engine/EditorBlueprintResources/StandardMacros.IncrementInt` (`self.CurrentSampleIDX`))
    (:`  `
      (if (>= _result (`KismetArrayLibrary.Array_Length` (`self.Samples`)))
        (set `self.CurrentSampleIDX` 0))
      (`AudioComponent.SetSound` (`self.Audio`) (`|GetArrayItem` (`self.Samples`) (`self.CurrentSampleIDX`)))
      (`KismetMathLibrary.LinearColor_SetRandomHue` _color)
      (`MaterialInstanceDynamic.SetVectorParameterValue` (`self.DynMaterial`) "EmissiveColor" (* _color 100.0))
      (bind _name (`self.GetSampleName`))
      (`/Game/Blueprints/BP_SampleTextActor.SetText` (`self.TextActor`) _name))))

(fn `Pause`
  (params (Pause :type Boolean))
  (`AudioComponent.SetPaused` (`self.Audio`) Pause))

(fn `PreviousSample`
  (bind _color (`self.Color`))
  (bind _result (`/Engine/EditorBlueprintResources/StandardMacros.DecrementInt` (`self.CurrentSampleIDX`))
    (:`  `
      (if (< _result 0)
        (set `self.CurrentSampleIDX` (- (`KismetArrayLibrary.Array_Length` (`self.Samples`)) 1)))
      (`AudioComponent.SetSound` (`self.Audio`) (`|GetArrayItem` (`self.Samples`) (`self.CurrentSampleIDX`)))
      (`KismetMathLibrary.LinearColor_SetRandomHue` _color)
      (`MaterialInstanceDynamic.SetVectorParameterValue` (`self.DynMaterial`) "EmissiveColor" (* _color 100.0))
      (bind _name (`self.GetSampleName`))
      (`/Game/Blueprints/BP_SampleTextActor.SetText` (`self.TextActor`) _name))))

(fn `UserConstructionScript`)